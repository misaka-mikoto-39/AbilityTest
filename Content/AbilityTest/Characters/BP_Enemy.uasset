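; BP_Enemy is an enemy character Blueprint that shows its health on an attached widget.
; Its OnHealthChange event casts the HealthBar component's widget to WBP_HealthBar and passes it health divided by max health as the fill percentage.
; The other events are disabled stubs and the construction script only calls the parent, so this graph holds no other behavior.
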(event `self.BP_OnHealthChange`
  (params (Health :type "Float (single-precision)") (MaxHealth :type "Float (single-precision)"))
  (bind _aswbp_health_bar (cast `/Game/AbilityTest/UI/WBP_HealthBar` (`WidgetComponent.GetUserWidgetObject` (`self.HealthBar`))))
  (`/Game/AbilityTest/UI/WBP_HealthBar.SetHealthPercentage` _aswbp_health_bar (/ Health MaxHealth)))

(fn `UserConstructionScript`
  (`parent.UserConstructionScript`))