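; GA_InseinNebia is a gameplay ability that plays a cast animation and spawns a mist Niagara effect at the player character.
; On activation it runs the parent logic, commits the ability, starts the UI cooldown and plays the health regen cast montage.
; Every montage outcome, including interruption or cancellation, spawns NS_Mist at the BP_PlayerCharacter's location and ends the ability.
; The graph itself applies no gameplay effect.
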(event `self.K2_ActivateAbility`
  (`parent.K2_ActivateAbility`)
  (`self.K2_CommitAbility`)
  (`self.Do UI Cooldown`)
  (`AbilityTask_PlayMontageAndWait.CreatePlayMontageAndWaitProxy` "None" "/Game/AbilityTest/Characters/Animations/AM_Cast_HealthRegen.AM_Cast_HealthRegen"
    (:`OnCompleted`
      _)
    (:`OnBlendOut`
      _)
    (:`OnInterrupted`
      _)
    (:`OnCancelled`
      _))
  (bind _asbp_player_character (cast `/Game/AbilityTest/Characters/BP_PlayerCharacter` (`self.GetOwningActorFromActorInfo`))
    (:`then`
      (`NiagaraFunctionLibrary.SpawnSystemAtLocation` "/Game/AbilityTest/Characters/GameplayAbilities/InseinNebia/FX/NS_Mist.NS_Mist" (`Actor.K2_GetActorLocation` _asbp_player_character))
      (`self.K2_EndAbility`))
    (:`CastFailed`
      (`self.K2_EndAbility`))))