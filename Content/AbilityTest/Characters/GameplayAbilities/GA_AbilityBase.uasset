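; Base Gameplay Ability Blueprint that provides shared helpers, with no activation logic of its own.
; GetCharacterBase casts the owning actor and its controller to BP_GameCharacter and BP_PlayerController for the other helpers.
; DoUICooldown starts the cooldown on the player UI slot matching this ability's class.
; IsCostStillAvaliable compares Health, Mana or Strength against the negated ability cost, requiring Health to stay strictly above it.
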(fn `Do UI Cooldown`
  (bind (_character _controller) (`self.GetCharacterBase`))
  (`/Engine/EditorBlueprintResources/StandardMacros.IsValid` _controller
    (:`Is Valid`
      (for _array_element (`/Game/AbilityTest/UI/WBP_PrimaryUI.Slots` (`/Game/AbilityTest/Characters/BP_PlayerController.PrimaryUI` _controller))
        (bind _returnvalue (`self.GetAbilityInfo`))
        (bind (_abilityinfo_cooldownduration _abilityinfo_cost _abilityinfo_uimaterial _abilityinfo_costtype _abilityinfo_abilityclass) (break `GameplayAbilityInfo` (`/Game/AbilityTest/UI/WBP_Ability_Slot.AbilityInfo` _array_element)))
        (if (== _abilityinfo_abilityclass (`.AbilityClass` (break `GameplayAbilityInfo` _returnvalue)))
          (`/Game/AbilityTest/UI/WBP_Ability_Slot.StartCooldown` _array_element)
          (return))))))

(fn `GetCharacterBase`
  (returns (Character :type "/Game/AbilityTest/Characters/BP_GameCharacter Object Reference") (Controller :type "/Game/AbilityTest/Characters/BP_PlayerController Object Reference"))
  (bind _asbp_game_character (cast `/Game/AbilityTest/Characters/BP_GameCharacter` (`self.GetOwningActorFromActorInfo`)))
  (bind _asbp_player_controller (cast `/Game/AbilityTest/Characters/BP_PlayerController` (`Pawn.GetController` _asbp_game_character)))
  (return _asbp_game_character _asbp_player_controller))

(fn `IsCostStillAvaliable`
  (returns (IsAvaliable :type Boolean))
  (bind _returnvalue (`self.GetAbilityInfo`))
  (switch `EAbilityCostType` (`.CostType` (break `GameplayAbilityInfo` _returnvalue))
    (:`Health`
      (bind _character (`self.GetCharacterBase`))
      (bind (_health_basevalue _health_currentvalue) (break `GameplayAttributeData` (`BaseAttributeSet.Health` (`GameCharacter.BaseAttributeSetComp` _character))))
      (bind _returnvalue_2 (* (`.Cost` (break `GameplayAbilityInfo` _returnvalue)) -1.0))
      (return (> _health_currentvalue _returnvalue_2)))
    (:`Mana`
      (bind _character_2 (`self.GetCharacterBase`))
      (bind (_mana_basevalue _mana_currentvalue) (break `GameplayAttributeData` (`BaseAttributeSet.Mana` (`GameCharacter.BaseAttributeSetComp` _character_2))))
      (return (>= _mana_currentvalue _returnvalue_2)))
    (:`Strength`
      (bind _character_3 (`self.GetCharacterBase`))
      (bind (_strength_basevalue _strength_currentvalue) (break `GameplayAttributeData` (`BaseAttributeSet.Strength` (`GameCharacter.BaseAttributeSetComp` _character_3))))
      (return (>= _strength_currentvalue _returnvalue_2)))))