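; Gameplay Ability that dashes the player character forward, in a file marked as old by its name.
; On activation it commits, saves and zeroes the character's ground friction, then applies a velocity-change impulse along the actor's forward vector.
; A dash montage times the ability: completion, blend-out, interruption or cancellation restores the saved friction and ends it.
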(event `self.K2_ActivateAbility`
  (`self.K2_CommitAbility`)
  (bind _asbp_player_character (cast `/Game/AbilityTest/Characters/BP_PlayerCharacter` (`self.GetOwningActorFromActorInfo`))
    (:`then`
      (bind _charactermovement (`Character.CharacterMovement` _asbp_player_character))
      (set `self.Original Ground Friction` (`CharacterMovementComponent.GroundFriction` _charactermovement))
      (set `CharacterMovementComponent.GroundFriction` 0.0 _charactermovement)
      (`CharacterMovementComponent.AddImpulse` _charactermovement (* (`Actor.GetActorForwardVector` _asbp_player_character) 2000.0) true)
      (`AbilityTask_PlayMontageAndWait.CreatePlayMontageAndWaitProxy` "None" "/Game/AbilityTest/Characters/Animations/AM_Ability_Dash.AM_Ability_Dash"
        (:`OnCompleted`
          _)
        (:`OnBlendOut`
          _)
        (:`OnInterrupted`
          _)
        (:`OnCancelled`
          _))
      (`|ExecutionSequence`
        (:`then_0`
          (set `CharacterMovementComponent.GroundFriction` (`self.Original Ground Friction`) _charactermovement)
          (`self.K2_EndAbility`))))
    (:`CastFailed`
      (`self.K2_EndAbility`))))