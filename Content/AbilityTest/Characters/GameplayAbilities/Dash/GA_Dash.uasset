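; GA_Dash is a gameplay ability that dashes the player character forward.
; On activation it commits, casts the avatar to BP_PlayerCharacter, and plays the dash montage while applying an additive constant root motion force along the horizontal forward vector.
; The force clamps exit velocity, and the ability ends after a short delay, or immediately if the cast fails.
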(event `self.K2_ActivateAbility`
  (`self.K2_CommitAbility`)
  (bind _asbp_player_character (cast `/Game/AbilityTest/Characters/BP_PlayerCharacter` (`self.GetOwningActorFromActorInfo`))
    (:`then`
      (`AbilityTask_PlayMontageAndWait.CreatePlayMontageAndWaitProxy` "None" "/Game/AbilityTest/Characters/Animations/AM_Ability_Dash.AM_Ability_Dash"
        (:`then`
          (`AbilityTask_ApplyRootMotionConstantForce.ApplyRootMotionConstantForce` "None" (`KismetMathLibrary.Normal` (* (`Actor.GetActorForwardVector` _asbp_player_character) (1.0 1.0 0.0))) 3000.0 0.25 true null "ClampVelocity" (0.0 0.0 0.0) 1000.0
            (:`then`
              (`KismetSystemLibrary.Delay` 0.3)
              (`self.K2_EndAbility`))))
        (:`OnCompleted`)
        (:`OnBlendOut`)
        (:`OnInterrupted`)
        (:`OnCancelled`)))
    (:`CastFailed`
      (`self.K2_EndAbility`))))