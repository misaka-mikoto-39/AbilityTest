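; Fire Blast gameplay ability that commits, triggers the UI cooldown and plays a cast montage, ending when the montage ends.
; Montage-timed Pull and Push gameplay events are awaited in sequence, each running instant area targeting through GATargetActorGetAround.
; Only the Push targets receive the damage effect; the Pull target data is unused, with its damage and debug-print nodes left disconnected.
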(event `self.K2_ActivateAbility`
  (`self.K2_CommitAbility`)
  (`self.Do UI Cooldown`)
  (`AbilityTask_PlayMontageAndWait.CreatePlayMontageAndWaitProxy` "None" "/Game/AbilityTest/Characters/Animations/AM_FireBlast_Cast.AM_FireBlast_Cast"
    (:`then`
      (`AbilityTask_WaitGameplayEvent.WaitGameplayEvent` (struct :`TagName` "Skill.FireBlast.Pull") null
        (:`EventReceived`
          (bind (_asynctaskproxy _data) (`AbilityTask_WaitTargetData.WaitTargetData` "None" "Instant" "/Script/AbilityTest.GATargetActorGetAround" 300.0 (struct) (struct) null)
            (:`then`
              (`AbilityTask_WaitGameplayEvent.WaitGameplayEvent` (struct :`TagName` "Skill.FireBlast.Push") null
                (:`EventReceived`
                  (bind (_asynctaskproxy_2 _data_2) (`AbilityTask_WaitTargetData.WaitTargetData` "None" "Instant" "/Script/AbilityTest.GATargetActorGetAround" 300.0 (struct) (struct) null)
                    (:`ValidData`
                      (`self.BP_ApplyGameplayEffectToTarget` _data_2 "/Game/AbilityTest/Characters/GameplayAbilities/FireBlast/GE_FireBlast_Damage.GE_FireBlast_Damage_C"))))))
            (:`Cancelled`
              (`self.K2_EndAbility`))))))
    (:`OnCompleted`
      (`self.K2_EndAbility` :!label _label))
    (:`OnBlendOut`
      (goto _label))
    (:`OnInterrupted`
      (goto _label))
    (:`OnCancelled`
      (goto _label))))