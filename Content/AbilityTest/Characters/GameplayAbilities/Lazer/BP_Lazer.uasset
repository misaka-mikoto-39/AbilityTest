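; BP_Lazer is a laser beam actor whose skeletal mesh stretches to match the distance to its EndPoint component.
; On BeginPlay it records the beam's original length from the actor's location to the mesh's "end" socket.
; Each tick it passes the difference between the EndPoint distance and that length to the mesh's Anim Blueprint as an X-axis EndBoneOffset.
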(event `self.ReceiveBeginPlay`
  (set `self.BeamOriginalLength` (`KismetMathLibrary.VSize` (- (`SceneComponent.GetSocketLocation` (`self.LazerMesh`) "end") (`self.K2_GetActorLocation`)))))

(event `self.ReceiveTick`
  (params (DeltaSeconds :type "Float (single-precision)"))
  (bind _aslazer_skeletal_mesh_skeleton_anim_blueprint (cast `/Game/AbilityTest/Characters/GameplayAbilities/Lazer/LazerAssets/lazer_skeletal_mesh_Skeleton_AnimBlueprint` (`SkeletalMeshComponent.GetAnimInstance` (`self.LazerMesh`))))
  (set `/Game/AbilityTest/Characters/GameplayAbilities/Lazer/LazerAssets/lazer_skeletal_mesh_Skeleton_AnimBlueprint.EndBoneOffset` (`KismetMathLibrary.MakeVector` (- (`KismetMathLibrary.VSize` (- (`SceneComponent.K2_GetComponentLocation` (`self.EndPoint`)) (`self.K2_GetActorLocation`))) (`self.BeamOriginalLength`))) _aslazer_skeletal_mesh_skeleton_anim_blueprint))

(fn `UserConstructionScript`)